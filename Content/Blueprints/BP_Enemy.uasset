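; BP_Enemy is a melee enemy that chases the player and reports to BP_WaveSpawner when it dies.
; A looping AIMoveTo plays a push montage in range, whose notify sphere-traces for pawns and applies damage.
; Damage knocks it back; at zero health it ragdolls, is destroyed after a delay, and asks the spawner to check for enemies.
; A random-roaming Wonder event exists but is not called here.
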(event Custom|Wonder
  ;[1 1 1] Wonder
  (AI|AIMoveTo self (.RandomLocation (AI|Navigation|GetRandomReachablePointinRadius (Transformation|GetActorLocation) 5e+02 0 0)) 0 5.0 false
    (:OnSuccess
      (Utilities|FlowControl|Delay 1.0)
      (CallFunction|Wonder))))

(event Custom|Chase%20Player
  (bind _attack_trace_pos (Variables|Default|GetAttack%20Trace%20Pos))
  (bind _returnvalue (Transformation|GetWorldLocation _attack_trace_pos))
  ;[1 1 1] Chase Player
  (AI|AIMoveTo self "0, 0, 0" (Game|GetPlayerCharacter 0) 5e+01 false
    (:OnSuccess
      (if (<= (Math|Vector|Distance(Vector) (Transformation|GetWorldLocation (Variables|Character|GetMesh self)) (Transformation|GetWorldLocation (Variables|/Script/Engine.Character|GetMesh (Game|GetPlayerCharacter 0)))) 2e+02)
        (Animation|Montage|PlayMontage (Variables|Character|GetMesh) "/Game/Characters/Mannequins/Animations/Manny/push_Montage.push_Montage"
          (:OnCompleted
            (Utilities|FlowControl|Delay 1.0)
            (CallFunction|ChasePlayer :!label _label))
          (:OnNotifyBegin
            (bind (_outhit _returnvalue_2) (Collision|SphereTraceForObjects _returnvalue (+ _returnvalue (* (Math|Vector|GetForwardVector _attack_trace_pos) 5e+01)) 25.0 (Utilities|Array|MakeArray "ObjectTypeQuery3") false 0 "ForDuration"))
            (if _returnvalue_2
              (Game|Damage|ApplyDamage (.HitActor (Collision|BreakHitResult _outhit)) 1e+01 0 0))))
        (else
          (goto _label))))))

(event Game|Damage|EventAnyDamage
  (params (Damage :type Float%20%28single-precision%29) (DamageType :type Damage%20Type%20Object%20Reference) (InstigatedBy :type Controller%20Object%20Reference) (DamageCauser :type Actor%20Object%20Reference))
  ;[1 1 1] Damage
  (Variables|Default|SetHealth (- (Variables|Default|GetHealth) Damage))
  (if (<= (Variables|Default|GetHealth) 0.0)
    (Variables|Default|SetCan%20Attack false)
    (Physics|SetSimulatePhysics (Variables|Character|GetMesh) true)
    (Pawn|Components|CharacterMovement|DisableMovement (Variables|Character|GetCharacterMovement))
    (Utilities|FlowControl|Delay 3.0)
    (Actor|DestroyActor)
    (bind _returnvalue (Actor|GetActorOfClass "/Game/Blueprints/BP_WaveSpawner.BP_WaveSpawner_C"))
    (Default|CheckforEnemies _returnvalue)
    (else
      (Character|LaunchCharacter (+ (* (Transformation|GetActorForwardVector) -2e+02) (* (Transformation|GetActorUpVector) 1e+02)) false false))))

(event EventBeginPlay
  (CallFunction|ChasePlayer))

(fn ConstructionScript)